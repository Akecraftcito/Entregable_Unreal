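; Damage hazard actor that takes a fixed amount of VidaActual (health) from BP_ThirdPersonCharacter when it overlaps the Box.
; Surviving characters jump; otherwise the Game Over widget opens with UI-only input and cursor, and the character is destroyed.
; The death check re-evaluates the clamped subtraction after the health update, so it triggers one hit before health reaches zero.
; Two older copies of the logic remain unconnected.
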(event `self.Box.OnComponentBeginOverlap`
  (params (OverlappedComponent :type "PrimitiveComponent Object Reference") (OtherActor :type "Actor Object Reference") (OtherComp :type "PrimitiveComponent Object Reference") (OtherBodyIndex :type Integer) (bFromSweep :type Boolean) (SweepResult :type "HitResult Structure (by ref)"))
  (bind _returnvalue (`GameplayStatics.GetPlayerController` 0))
  (bind _asbp_third_person_character (cast `/Game/ThirdPerson/Blueprints/BP_ThirdPersonCharacter` OtherActor))
  (bind _output_get (set `self.As BP Third Person Character` _asbp_third_person_character))
  (bind _returnvalue_2 (`KismetMathLibrary.FClamp` (- (`/Game/ThirdPerson/Blueprints/BP_ThirdPersonCharacter.VidaActual` _output_get) 20.0) 0.0 (`/Game/ThirdPerson/Blueprints/BP_ThirdPersonCharacter.VidaTotal` _output_get)))
  (set `/Game/ThirdPerson/Blueprints/BP_ThirdPersonCharacter.VidaActual` _returnvalue_2 _output_get)
  (if (<= _returnvalue_2 0.0)
    (bind _returnvalue_3 (`|CreateWidget` "/Game/Blueprints/WB_Menu_Game_Over.WB_Menu_Game_Over_C"))
    (`UserWidget.AddToViewport` _returnvalue_3 0)
    (`WidgetBlueprintLibrary.SetInputMode_UIOnlyEx` _returnvalue _returnvalue_3)
    (set `PlayerController.bShowMouseCursor` true _returnvalue)
    (`self.K2_DestroyActor` _output_get)
    (else
      (`Character.Jump` _output_get))))

(fn `UserConstructionScript`)